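; Alice tower character Blueprint, a child class that drives its attack material effect and socket-bound body and hand particles.
; Attack begin and end events switch the "Attack" scalar on the dynamic material on and off.
; When a montage ends, it unhides the root, body and four hand effect components and sets a flag.
; While that flag is set, Tick calls BindParticle each frame, pairing the body and hand sockets with Root.
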(event Custom|AttackBegin_1
  ;[1 0 0] Attack
  (Utilities|IsValid (Variables|Default|GetMatDyn)
    (:Is%20Valid
      (Rendering|Material|SetScalarParameterValue (Variables|Default|GetMatDyn) "Attack" 1.0 :!class /Script/Engine.MaterialInstanceDynamic))))

(event Custom|AttackEnd_1
  ;[1 0 0] Attack
  (Utilities|IsValid (Variables|Default|GetMatDyn)
    (:Is%20Valid
      (Rendering|Material|SetScalarParameterValue (Variables|Default|GetMatDyn) "Attack" 0.0 :!class /Script/Engine.MaterialInstanceDynamic))))

(event EventBeginPlay
  ;[1 1 1] Init
  (|CallParentFunction))

(event Collision|EventActorBeginOverlap
  (params (OtherActor :type Actor%20Object%20Reference))
  (|CallParentFunction OtherActor) ; This node is disabled and will not be called.\nDrag off pins to build functionality.
)

(event EventTick
  (params (DeltaSeconds :type Float%20%28single-precision%29))
  ;[1 1 1] Comment
  (|CallParentFunction DeltaSeconds)
  (if (Variables|Default|GetbPlayMontage)
    (CallFunction|BindParticle (Variables|Default|GetPoint) "BodyPoint" "Root")
    (CallFunction|BindParticle (Variables|Default|GetHand_1) "Hand_1" "Root")
    (CallFunction|BindParticle (Variables|Default|GetHand_2) "Hand_2" "Root")
    (CallFunction|BindParticle (Variables|Default|GetHand_3) "Hand_3" "Root")
    (CallFunction|BindParticle (Variables|Default|GetHand_4) "Hand_4" "Root")))

(event EventOnMontageEnded
  (params (Montage :type Anim%20Montage%20Object%20Reference) (bInterrupted :type Boolean))
  ;[1 1 1] Init
  (Variables|Default|SetbPlayMontage true)
  (Development|SetHiddeninGame (Variables|Default|GetPoint) false false)
  (Development|SetHiddeninGame (Variables|Default|GetHand_1) false false)
  (Development|SetHiddeninGame (Variables|Default|GetHand_2) false false)
  (Development|SetHiddeninGame (Variables|Default|GetHand_3) false false)
  (Development|SetHiddeninGame (Variables|Default|GetHand_4) false false)
  (Development|SetHiddeninGame (Variables|Default|GetRootPoint) false false))

(fn ConstructionScript
  (|CallParentFunction))
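; Ball tower character that turns each tick along the direction from its AI controller's target to itself, so it faces away from the target.
; The TowersAIController_BP reference is cached shortly after BeginPlay.
; Once the montage-ended event fires, it shows the Line particle and rebinds it between R and L sockets each tick.
; Attack events toggle a dynamic-material refraction parameter, while AnimTag hides the line and sets the Death parameter.
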(event EventBeginPlay
  (|CallParentFunction)
  (Utilities|FlowControl|Delay 0.3)
  (bind _astowers_aicontroller_bp (Utilities|Casting|CastToTowersAIController_BP (Pawn|GetController)))
  (Variables|Default|SetRuleCharacterController _astowers_aicontroller_bp))

(event Collision|EventActorBeginOverlap
  (params (OtherActor :type Actor%20Object%20Reference))
  (|CallParentFunction OtherActor) ; This node is disabled and will not be called.\nDrag off pins to build functionality.
)

(event EventAnimTag
  (bind _matdyn (Variables|Default|GetMatDyn))
  (Development|SetHiddeninGame (Variables|Default|GetLine) true false)
  (Utilities|IsValid _matdyn
    (:Is%20Valid
      (Rendering|Material|SetScalarParameterValue _matdyn "Death" 1.0 :!class /Script/Engine.MaterialInstanceDynamic))))

(event EventCharacterDeath)

(event EventTick
  (params (DeltaSeconds :type Float%20%28single-precision%29))
  (bind _rulecharactercontroller (Variables|Default|GetRuleCharacterController))
  (bind _returnvalue (Class|RuleOftheAIController|GetTarget _rulecharactercontroller))
  (|CallParentFunction DeltaSeconds)
  (Utilities|FlowControl|Sequence
    (:then_0
      (Utilities|IsValid _rulecharactercontroller
        (:Is%20Valid
          (Utilities|IsValid _returnvalue
            (:Is%20Valid
              (Transformation|SetActorRotation (Math|Rotator|FindLookatRotation (Transformation|GetActorLocation _returnvalue) (Transformation|GetActorLocation))))))))
    (:then_1
      (if (Variables|Default|GetbPlayStartEnd)
        (CallFunction|BindParticle (Variables|Default|GetLine) "R" "L")))))

(event EventAttackBegin
  ;[1 0 0] Attack
  (Utilities|IsValid (Variables|Default|GetMatDyn)
    (:Is%20Valid
      (Rendering|Material|SetScalarParameterValue (Variables|Default|GetMatDyn) "BaseRefectFracionIn" 0.0 :!class /Script/Engine.MaterialInstanceDynamic))))

(event EventAttackEnd
  ;[1 0 0] Attack
  (Utilities|IsValid (Variables|Default|GetMatDyn)
    (:Is%20Valid
      (Rendering|Material|SetScalarParameterValue (Variables|Default|GetMatDyn) "BaseRefectFracionIn" -0.23 :!class /Script/Engine.MaterialInstanceDynamic))))

(event EventOnMontageEnded
  (params (Montage :type Anim%20Montage%20Object%20Reference) (bInterrupted :type Boolean))
  (Variables|Default|SetbPlayStartEnd true)
  (Development|SetHiddeninGame (Variables|Default|GetLine) false false))

(fn ConstructionScript
  (|CallParentFunction))